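; BP_TCP is a TCP client that links the game's VehicleManager to a local socket server.
; On BeginPlay it connects to a fixed localhost port, stores the connection ID and prints connect and disconnect events.
; Incoming messages are read whole as strings and passed to VehicleManager's LCEvent.
; A SendData function writes outgoing data over the stored connection, but nothing in this Blueprint calls it.
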(event `self.ReceiveBeginPlay`
  (bind _connectionid (`self.Connect` "127.0.0.1" 8800 (delegate `Disconnected`) (delegate `Connected`) (delegate `MessageReceived`)))
  (set `self.Connection Id` _connectionid))

(event `Disconnected`
  (params (ConnectionId :type Integer))
  (`KismetSystemLibrary.PrintString` "Server Disconnected"))

(event `Connected`
  (params (ConnectionId :type Integer))
  (`KismetSystemLibrary.PrintString` "Server Connected"))

(event `MessageReceived`
  (params (ConnectionId :type Integer) (Message :type "Array of Byte (by ref)"))
  (`self.Receive Data` Message))

(fn `Receive Data`
  (params (data :type "Array of Byte"))
  (bind _returnvalue (`self.Message_ReadString` data (`KismetArrayLibrary.Array_Length` data)))
  (`/Game/Blueprints/BP_VehicleManager.LCEvent` (`self.VehicleManager`) _returnvalue))

(fn `Send Data`
  (params (data :type "Array of Byte"))
  (bind _returnvalue (`self.SendData` (`self.Connection Id`) data))
  (if _returnvalue
    _))

(fn `UserConstructionScript`)