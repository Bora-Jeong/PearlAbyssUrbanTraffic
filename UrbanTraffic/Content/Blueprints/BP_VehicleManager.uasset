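; BP_VehicleManager gathers every AI_Car_Source actor at BeginPlay and streams their per-frame data out through a TCP server.
; Each tick it first has every vehicle record its current velocity for the frame count, then in a second pass concatenates each vehicle's info string.
; The combined string is converted to bytes and sent in one SendData call.
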(event `self.ReceiveBeginPlay`
  (bind _outactors (`GameplayStatics.GetAllActorsOfClass` "/Game/AITraffic/AI_Car_Source.AI_Car_Source_C"))
  (set `self.Vehicles` _outactors))

(event `self.ReceiveTick`
  (params (DeltaSeconds :type "Float (single-precision)"))
  (set `self.Frame` (`KismetSystemLibrary.GetFrameCount`))
  (set `self.Info` "")
  (for _array_element (`self.Vehicles`)
    (`/Game/AITraffic/AI_Car_Source.Record Current Velocity` _array_element (`self.Frame`)))
  (for _array_element_2 (`self.Vehicles`)
    (bind _output (`/Game/AITraffic/AI_Car_Source.Get Info` _array_element_2 (`self.Frame`)))
    (set `self.Info` (`KismetStringLibrary.Concat_StrStr` (`self.Info`) _output)))
  (`/Game/Blueprints/BP_TCP.Send Data` (`self.TCP Server`) (`TcpSocketConnection.Conv_StringToBytes` (`self.Info`))))

(fn `UserConstructionScript`)