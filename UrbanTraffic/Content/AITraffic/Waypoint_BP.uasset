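; Waypoint actor for AI traffic that links to a next waypoint and can act as a vehicle removal point.
; Its construction script optionally draws a debug line to a valid NextWaypoint to show the link.
; With RemoveVehicles set, Tick uses a Delay to throttle a scan of all WheeledVehicle actors, destroying any within RemoveVehicleRadius.
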(event `self.ReceiveTick`
  (params (DeltaSeconds :type "Float (single-precision)"))
  (`KismetSystemLibrary.Delay` 0.6)
  (if (`self.RemoveVehicles?`)
    (bind _outactors (`GameplayStatics.GetAllActorsOfClass` "/Script/PhysXVehicles.WheeledVehicle"))
    (for _array_element _outactors
      (if (<= (`self.GetDistanceTo` _array_element) (`self.RemoveVehicleRadius`))
        (`self.K2_DestroyActor` _array_element)))))

(fn `UserConstructionScript`
  (bind _nextwaypoint (`self.NextWaypoint`))
  (if (`self.UseDebugLine?`)
    (`/Engine/EditorBlueprintResources/StandardMacros.IsValid` _nextwaypoint
      (:`Is Valid`
        (`KismetSystemLibrary.DrawDebugLine` (`self.K2_GetActorLocation` self) (`self.K2_GetActorLocation` _nextwaypoint) (struct :`R` 1.0 :`G` 0.699787 :`A` 1.0) (`self.BugLineDuration`) (`self.BugLineThickness`))))))