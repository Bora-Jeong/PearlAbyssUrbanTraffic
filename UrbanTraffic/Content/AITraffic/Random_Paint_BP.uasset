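; Editor utility actor that assigns random paint materials to AI traffic cars in the level.
; Its construction script treats the RandomizePaint boolean as a one-shot trigger, finding all AI_Car_Source actors, optionally filtered by tag, then clearing the flag.
; PaintCar sets a random entry from the PaintMaterials array on the configured material slot of each car's mesh.
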(fn `PaintCar`
  (params (CarBody :type "WheeledVehicle Object Reference"))
  (bind _paintmaterials (`self.PaintMaterials`))
  (`PrimitiveComponent.SetMaterial` (`WheeledVehicle.Mesh` CarBody) (`self.ElementNumber`) (`|GetArrayItem` _paintmaterials (`KismetMathLibrary.RandomIntegerInRange` 0 (- (`KismetArrayLibrary.Array_Length` _paintmaterials) 1)))))

(fn `UserConstructionScript`
  (if (`self.RandomizePaint?`)
    (if (`self.UseTag?`)
      (bind _outactors (`GameplayStatics.GetAllActorsOfClass` "/Game/AITraffic/AI_Car_Source.AI_Car_Source_C"))
      (for _array_element _outactors
        (if (`self.ActorHasTag` _array_element (`self.TagName`))
          (`self.PaintCar` _array_element)))
      (set `self.RandomizePaint?` false)
      (else
        (bind _outactors_2 (`GameplayStatics.GetAllActorsOfClass` "/Game/AITraffic/AI_Car_Source.AI_Car_Source_C"))
        (for _array_element_2 _outactors_2
          (`self.PaintCar` _array_element_2))
        (set `self.RandomizePaint?` false)))))