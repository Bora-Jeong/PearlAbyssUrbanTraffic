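; Traffic light for AI traffic that cycles through green, yellow, red and optional turn signals, or flashes yellow without a master.
; In the Construction Script, the master links up to three lights and copies its settings to them.
; Tick runs a DoOnce/Delay state machine driving dynamic material intensities, forcing third and fourth lights red during master green.
; Without splines, red states activate vehicle stop collision boxes.
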(event `self.ReceiveBeginPlay`)

(event `self.ReceiveTick`
  (params (DeltaSeconds :type "Float (single-precision)"))
  ;[1 1 1] If no master exist, caution flash.
  (if (== (`self.FirstLightMaster`) null)
    (`KismetSystemLibrary.Delay` 0.5)
    (`/Engine/EditorBlueprintResources/StandardMacros.FlipFlop`
      (:`A`
        (`self.SetTrafficLightColors` "Yellow"))
      (:`B`
        (`self.SetTrafficLightColors` "None")))
    (else
      (`self.EastAndWestCycle`) ; Setup East and West Traffic Lights.
      (if (not (`self.UseSplines?`))
        (`self.CollisionBoxActivity`) ; Use collision boxes.
      )
      (set `self.LightStatus` (select `int` (`self.NextLight`) :`0` "Green" :`1` "Yellow" :`2` "Red" :`3` "TurnGreen" :`4` "TurnYellow" :`5` "TurnRed" :!type "Name"))
      (switch `int` (`self.NextLight`)
        (:`0`
          ;[1 1 1] Light cycle.
          (`/Engine/EditorBlueprintResources/StandardMacros.DoOnce` false :!label _label
            (:`Completed`
              (`self.SetTrafficLightColors` (`self.LightStatus`))
              (set `self.RedLightActive?` false)
              (set `self.TurnRedLightActive?` true)
              (`KismetSystemLibrary.Delay` (- (`self.LightDuration`) (`self.YellowLightDuration`)))
              (set `self.NextLight` 1)
              (goto _label :!via `Reset`))))
        (:`1`
          (`/Engine/EditorBlueprintResources/StandardMacros.DoOnce` false :!label _label_2
            (:`Completed`
              (`self.SetTrafficLightColors` (`self.LightStatus`))
              (set `self.RedLightActive?` true)
              (set `self.TurnRedLightActive?` true)
              (`KismetSystemLibrary.Delay` (`self.YellowLightDuration`))
              (set `self.NextLight` 2)
              (goto _label_2 :!via `Reset`))))
        (:`2`
          (`/Engine/EditorBlueprintResources/StandardMacros.DoOnce` false :!label _label_3
            (:`Completed`
              (`self.SetTrafficLightColors` (`self.LightStatus`))
              (set `self.RedLightActive?` true)
              (set `self.TurnRedLightActive?` true)
              (`KismetSystemLibrary.Delay` (+ (`self.LightDuration`) (`self.TrafficLightDelay`)))
              (if (`self.UseTurnSignals?`)
                (set `self.NextLight` 3)
                (goto _label_3 :!via `Reset`)
                (else
                  (set `self.NextLight` 0)
                  (goto _label_3 :!via `Reset`))))))
        (:`3`
          ;[1 1 1] Turn signal light cycle.
          (`/Engine/EditorBlueprintResources/StandardMacros.DoOnce` false :!label _label_4
            (:`Completed`
              (`self.SetTrafficLightColors` (`self.LightStatus`))
              (set `self.TurnRedLightActive?` false)
              (`KismetSystemLibrary.Delay` (- (`self.TurnLightDuration`) (`self.YellowLightDuration`)))
              (set `self.NextLight` 4)
              (goto _label_4 :!via `Reset`))))
        (:`4`
          (`/Engine/EditorBlueprintResources/StandardMacros.DoOnce` false :!label _label_5
            (:`Completed`
              (`self.SetTrafficLightColors` (`self.LightStatus`))
              (set `self.TurnRedLightActive?` true)
              (`KismetSystemLibrary.Delay` (`self.YellowLightDuration`))
              (set `self.NextLight` 5)
              (goto _label_5 :!via `Reset`))))
        (:`5`
          (`/Engine/EditorBlueprintResources/StandardMacros.DoOnce` false :!label _label_6
            (:`Completed`
              (`self.SetTrafficLightColors` (`self.LightStatus`))
              (set `self.TurnRedLightActive?` true)
              (`KismetSystemLibrary.Delay` (+ (+ (`self.TurnLightDuration`) (`self.YellowLightDuration`)) (`self.TrafficLightDelay`)))
              (set `self.NextLight` 0)
              (goto _label_6 :!via `Reset`))))))))

(fn `AutoSync`
  (params (TrafficLight :type "/Game/AITraffic/TrafficLight_BP Object Reference") (LightDuration :type "Float (double-precision)") (YellowLightDuration :type "Float (double-precision)") (TurnLightDuration :type "Float (double-precision)") (TrafficLightIntensity :type "Float (double-precision)") (TrafficLightDelay :type "Float (double-precision)") (RedLightMaterialID :type Integer) (YellowLightMaterialID :type Integer) (GreenLightMaterialID :type Integer) (TurnRedLightMaterialID :type Integer) (TurnYellowLightMaterialID :type Integer) (TurnGreenLightMaterialID :type Integer) (RedLightMaterialSource :type "MaterialInterface Object Reference") (YellowLightSource :type "MaterialInterface Object Reference") (GreenLightSource :type "MaterialInterface Object Reference") (TurnRedLightMaterialSource :type "MaterialInterface Object Reference") (TurnYellowLightSource :type "MaterialInterface Object Reference") (TurnGreenLightSource :type "MaterialInterface Object Reference"))
  (set `/Game/AITraffic/TrafficLight_BP.LightDuration` LightDuration TrafficLight)
  (set `/Game/AITraffic/TrafficLight_BP.YellowLightDuration` YellowLightDuration TrafficLight)
  (set `/Game/AITraffic/TrafficLight_BP.TurnLightDuration` TurnLightDuration TrafficLight)
  (set `/Game/AITraffic/TrafficLight_BP.TrafficLightIntensity` TrafficLightIntensity TrafficLight)
  (set `/Game/AITraffic/TrafficLight_BP.TrafficLightDelay` TrafficLightDelay TrafficLight)
  (set `/Game/AITraffic/TrafficLight_BP.RedLightMaterialID` RedLightMaterialID TrafficLight)
  (set `/Game/AITraffic/TrafficLight_BP.YellowLightMaterialID` YellowLightMaterialID TrafficLight)
  (set `/Game/AITraffic/TrafficLight_BP.GreenLightMaterialID` GreenLightMaterialID TrafficLight)
  (set `/Game/AITraffic/TrafficLight_BP.TurnRedLightMaterialID` TurnRedLightMaterialID TrafficLight)
  (set `/Game/AITraffic/TrafficLight_BP.TurnYellowLightMaterialID` TurnYellowLightMaterialID TrafficLight)
  (set `/Game/AITraffic/TrafficLight_BP.TurnGreenLightMaterialID` TurnGreenLightMaterialID TrafficLight)
  (set `/Game/AITraffic/TrafficLight_BP.RedLightMaterialSource` RedLightMaterialSource TrafficLight)
  (set `/Game/AITraffic/TrafficLight_BP.YellowLightSource` YellowLightSource TrafficLight)
  (set `/Game/AITraffic/TrafficLight_BP.GreenLightSource` GreenLightSource TrafficLight)
  (set `/Game/AITraffic/TrafficLight_BP.TurnRedLightMaterialSource` TurnRedLightMaterialSource TrafficLight)
  (set `/Game/AITraffic/TrafficLight_BP.TurnYellowLightSource` TurnYellowLightSource TrafficLight)
  (set `/Game/AITraffic/TrafficLight_BP.TurnGreenLightSource` TurnGreenLightSource TrafficLight))

(fn `CollisionBoxActivity`
  (bind _mainvehiclecollisionbox (`self.MainVehicleCollisionBox`))
  (bind _turnvehiclecollisionbox (`self.TurnVehicleCollisionBox`))
  (bind _mainvehiclecollisionbox_2 (`self.MainVehicleCollisionBox`))
  (bind _turnvehiclecollisionbox_2 (`self.TurnVehicleCollisionBox`))
  (`|ExecutionSequence`
    (:`then_0`
      (if (`self.RedLightActive?`)
        (`ActorComponent.SetActive` _mainvehiclecollisionbox_2 true false)
        (else
          (`ActorComponent.SetActive` _mainvehiclecollisionbox_2 false false)))
      (if (`self.UseTurnSignals?`)
        (if (`self.TurnRedLightActive?`)
          (`ActorComponent.SetActive` _turnvehiclecollisionbox_2 true false)
          (else
            (`ActorComponent.SetActive` _turnvehiclecollisionbox_2 false false)))))
    (:`then_1`
      (`/Engine/EditorBlueprintResources/StandardMacros.DoOnce` false ; Enable main collision.
        (:`Completed`
          (if (`self.UseSplines?`)
            (`PrimitiveComponent.SetCollisionEnabled` _mainvehiclecollisionbox "NoCollision") ; If spline is enabled, disable collsion boxes.
            (if (`self.UseTurnSignals?`)
              (`PrimitiveComponent.SetCollisionEnabled` _turnvehiclecollisionbox "NoCollision") ; If spline is enabled, disable collsion boxes.
              (else
                (`PrimitiveComponent.SetCollisionEnabled` _turnvehiclecollisionbox "QueryOnly") ; If spline is enabled, disable collsion boxes.
              ))
            (else
              (`PrimitiveComponent.SetCollisionEnabled` _mainvehiclecollisionbox "QueryOnly") ; If spline is enabled, disable collsion boxes.
            )))))))

(fn `DrawDebugLine`
  (params (TrafficLight :type "/Game/AITraffic/TrafficLight_BP Object Reference"))
  (if (`self.UseDebugLine?`)
    (`/Engine/EditorBlueprintResources/StandardMacros.IsValid` TrafficLight
      (:`Is Valid`
        (`KismetSystemLibrary.DrawDebugLine` (`self.K2_GetActorLocation` (`self.FirstLightMaster`)) (`self.K2_GetActorLocation` TrafficLight) (struct :`G` 1.0 :`B` 0.008223 :`A` 1.0) (`self.BugLineDuration`) (`self.BugLineThickness`))))))

(fn `EastAndWestCycle`
  (if (or (== (`self.ThirdLight`) self) (== (`self.ForthLight`) self))
    (if (== (`/Game/AITraffic/TrafficLight_BP.NextLight` (`self.FirstLightMaster`)) 0)
      (set `self.NextLight` 2))))

(fn `SetTrafficLightColors`
  (params (Name :type Name))
  (if (== Name "Red")
    (`MaterialInstanceDynamic.SetScalarParameterValue` (`self.RedLightMaterial`) "LightIntensity" (`self.TrafficLightIntensity`))
    (`MaterialInstanceDynamic.SetScalarParameterValue` (`self.YellowLightMaterial`) "LightIntensity" 0.0)
    (`MaterialInstanceDynamic.SetScalarParameterValue` (`self.GreenLightMaterial`) "LightIntensity" 0.0)
    (`MaterialInstanceDynamic.SetScalarParameterValue` (`self.TurnRedLightMaterial`) "LightIntensity" (`self.TrafficLightIntensity`))
    (`MaterialInstanceDynamic.SetScalarParameterValue` (`self.TurnYellowLightMaterial`) "LightIntensity" 0.0)
    (`MaterialInstanceDynamic.SetScalarParameterValue` (`self.TurnGreenLightMaterial`) "LightIntensity" 0.0)
    (elif (== Name "Yellow")
      (`MaterialInstanceDynamic.SetScalarParameterValue` (`self.RedLightMaterial`) "LightIntensity" 0.0)
      (`MaterialInstanceDynamic.SetScalarParameterValue` (`self.YellowLightMaterial`) "LightIntensity" (`self.TrafficLightIntensity`))
      (`MaterialInstanceDynamic.SetScalarParameterValue` (`self.GreenLightMaterial`) "LightIntensity" 0.0)
      (`MaterialInstanceDynamic.SetScalarParameterValue` (`self.TurnRedLightMaterial`) "LightIntensity" (`self.TrafficLightIntensity`))
      (`MaterialInstanceDynamic.SetScalarParameterValue` (`self.TurnYellowLightMaterial`) "LightIntensity" 0.0)
      (`MaterialInstanceDynamic.SetScalarParameterValue` (`self.TurnGreenLightMaterial`) "LightIntensity" 0.0)
      (elif (== Name "Green")
        (`MaterialInstanceDynamic.SetScalarParameterValue` (`self.RedLightMaterial`) "LightIntensity" 0.0)
        (`MaterialInstanceDynamic.SetScalarParameterValue` (`self.YellowLightMaterial`) "LightIntensity" 0.0)
        (`MaterialInstanceDynamic.SetScalarParameterValue` (`self.GreenLightMaterial`) "LightIntensity" (`self.TrafficLightIntensity`))
        (`MaterialInstanceDynamic.SetScalarParameterValue` (`self.TurnRedLightMaterial`) "LightIntensity" (`self.TrafficLightIntensity`))
        (`MaterialInstanceDynamic.SetScalarParameterValue` (`self.TurnYellowLightMaterial`) "LightIntensity" 0.0)
        (`MaterialInstanceDynamic.SetScalarParameterValue` (`self.TurnGreenLightMaterial`) "LightIntensity" 0.0)
        (elif (== Name "TurnRed")
          (`MaterialInstanceDynamic.SetScalarParameterValue` (`self.TurnRedLightMaterial`) "LightIntensity" (`self.TrafficLightIntensity`))
          (`MaterialInstanceDynamic.SetScalarParameterValue` (`self.TurnYellowLightMaterial`) "LightIntensity" 0.0)
          (`MaterialInstanceDynamic.SetScalarParameterValue` (`self.TurnGreenLightMaterial`) "LightIntensity" 0.0)
          (`MaterialInstanceDynamic.SetScalarParameterValue` (`self.RedLightMaterial`) "LightIntensity" (`self.TrafficLightIntensity`))
          (`MaterialInstanceDynamic.SetScalarParameterValue` (`self.YellowLightMaterial`) "LightIntensity" 0.0)
          (`MaterialInstanceDynamic.SetScalarParameterValue` (`self.GreenLightMaterial`) "LightIntensity" 0.0)
          (elif (== Name "TurnYellow")
            (`MaterialInstanceDynamic.SetScalarParameterValue` (`self.TurnRedLightMaterial`) "LightIntensity" 0.0)
            (`MaterialInstanceDynamic.SetScalarParameterValue` (`self.TurnYellowLightMaterial`) "LightIntensity" (`self.TrafficLightIntensity`))
            (`MaterialInstanceDynamic.SetScalarParameterValue` (`self.TurnGreenLightMaterial`) "LightIntensity" 0.0)
            (`MaterialInstanceDynamic.SetScalarParameterValue` (`self.RedLightMaterial`) "LightIntensity" (`self.TrafficLightIntensity`))
            (`MaterialInstanceDynamic.SetScalarParameterValue` (`self.YellowLightMaterial`) "LightIntensity" 0.0)
            (`MaterialInstanceDynamic.SetScalarParameterValue` (`self.GreenLightMaterial`) "LightIntensity" 0.0)
            (elif (== Name "TurnGreen")
              (`MaterialInstanceDynamic.SetScalarParameterValue` (`self.TurnRedLightMaterial`) "LightIntensity" 0.0)
              (`MaterialInstanceDynamic.SetScalarParameterValue` (`self.TurnYellowLightMaterial`) "LightIntensity" 0.0)
              (`MaterialInstanceDynamic.SetScalarParameterValue` (`self.TurnGreenLightMaterial`) "LightIntensity" (`self.TrafficLightIntensity`))
              (`MaterialInstanceDynamic.SetScalarParameterValue` (`self.RedLightMaterial`) "LightIntensity" (`self.TrafficLightIntensity`))
              (`MaterialInstanceDynamic.SetScalarParameterValue` (`self.YellowLightMaterial`) "LightIntensity" 0.0)
              (`MaterialInstanceDynamic.SetScalarParameterValue` (`self.GreenLightMaterial`) "LightIntensity" 0.0)
              (else
                (`MaterialInstanceDynamic.SetScalarParameterValue` (`self.RedLightMaterial`) "LightIntensity" 0.0)
                (`MaterialInstanceDynamic.SetScalarParameterValue` (`self.YellowLightMaterial`) "LightIntensity" 0.0)
                (`MaterialInstanceDynamic.SetScalarParameterValue` (`self.GreenLightMaterial`) "LightIntensity" 0.0)
                (`MaterialInstanceDynamic.SetScalarParameterValue` (`self.RedLightMaterial`) "LightIntensity" 0.0)
                (`MaterialInstanceDynamic.SetScalarParameterValue` (`self.YellowLightMaterial`) "LightIntensity" 0.0)
                (`MaterialInstanceDynamic.SetScalarParameterValue` (`self.GreenLightMaterial`) "LightIntensity" 0.0)))))))))

(fn `UserConstructionScript`
  (bind _mainvehiclecollisionbox (`self.MainVehicleCollisionBox`))
  (bind _secondlight (`self.SecondLight`))
  (bind _turnlight (`self.TurnLight`))
  (bind _thirdlight (`self.ThirdLight`))
  (bind _forthlight (`self.ForthLight`))
  (bind _northlightmastertemp (`self.NorthLightMasterTemp`))
  (bind _turnvehiclecollisionbox (`self.TurnVehicleCollisionBox`))
  (`|ExecutionSequence`
    (:`then_0`
      ;[0.4597 0.8277 1] Set material colors.
      (bind _returnvalue (`PrimitiveComponent.CreateDynamicMaterialInstance` (`self.TrafficLight`) (`self.RedLightMaterialID`) (`self.RedLightMaterialSource`) "None"))
      (set `self.RedLightMaterial` _returnvalue)
      (bind _returnvalue_2 (`PrimitiveComponent.CreateDynamicMaterialInstance` (`self.TrafficLight`) (`self.YellowLightMaterialID`) (`self.YellowLightSource`) "None"))
      (set `self.YellowLightMaterial` _returnvalue_2)
      (bind _returnvalue_3 (`PrimitiveComponent.CreateDynamicMaterialInstance` (`self.TrafficLight`) (`self.GreenLightMaterialID`) (`self.GreenLightSource`) "None"))
      (set `self.GreenLightMaterial` _returnvalue_3)
      (`|ExecutionSequence`
        (:`then_0`
          (`/Engine/EditorBlueprintResources/StandardMacros.IsValid` (`self.FirstLightMaster`) ; If there is no master, set lights to none.
            (:`Is Valid`
              (if (== (`self.FirstLightMaster`) self)
                (`|ExecutionSequence`
                  (:`then_0`
                    ;[1 1 1] Is master and adds traffic lights to temp.
                    (set `self.NorthLightMasterTemp` (`self.FirstLightMaster`))
                    (set `self.SouthLightTemp` (`self.SecondLight`))
                    (set `self.WestLightTemp` (`self.ThirdLight`))
                    (set `self.EastLightTemp` (`self.ForthLight`))
                    (`SceneComponent.SetVisibility` (`self.MasterText`) true false) ; Display "Master" text.
                  )
                  (:`then_1`
                    ;[1 1 1] Is master and links other traffic lights to master assignments.
                    (set `/Game/AITraffic/TrafficLight_BP.FirstLightMaster` (`self.FirstLightMaster`) (`self.SecondLight`))
                    (set `/Game/AITraffic/TrafficLight_BP.SecondLight` _secondlight _secondlight)
                    (set `/Game/AITraffic/TrafficLight_BP.ThirdLight` (`self.ThirdLight`) (`self.SecondLight`))
                    (set `/Game/AITraffic/TrafficLight_BP.ForthLight` (`self.ForthLight`) (`self.SecondLight`))
                    ;[1 0.09183 0.06198] Draw Debug line.
                    (`self.DrawDebugLine` (`self.SecondLight`))
                    ;[0.1374 0.3882 1] Auto Sync System
                    (`self.AutoSync` (`self.SecondLight`) (`self.LightDuration`) (`self.YellowLightDuration`) (`self.TurnLightDuration`) (`self.TrafficLightIntensity`) (`self.TrafficLightDelay`) (`self.RedLightMaterialID`) (`self.YellowLightMaterialID`) (`self.GreenLightMaterialID`) (`self.TurnRedLightMaterialID`) (`self.TurnYellowLightMaterialID`) (`self.TurnGreenLightMaterialID`) (`self.RedLightMaterialSource`) (`self.YellowLightSource`) (`self.GreenLightSource`) (`self.TurnRedLightMaterialSource`) (`self.TurnYellowLightSource`) (`self.TurnGreenLightSource`)))
                  (:`then_2`
                    (set `/Game/AITraffic/TrafficLight_BP.FirstLightMaster` (`self.FirstLightMaster`) (`self.ThirdLight`))
                    (set `/Game/AITraffic/TrafficLight_BP.SecondLight` (`self.SecondLight`) (`self.ThirdLight`))
                    (set `/Game/AITraffic/TrafficLight_BP.ThirdLight` _thirdlight _thirdlight)
                    (set `/Game/AITraffic/TrafficLight_BP.ForthLight` (`self.ForthLight`) (`self.ThirdLight`))
                    (`self.DrawDebugLine` (`self.ThirdLight`))
                    (`self.AutoSync` (`self.ThirdLight`) (`self.LightDuration`) (`self.YellowLightDuration`) (`self.TurnLightDuration`) (`self.TrafficLightIntensity`) (`self.TrafficLightDelay`) (`self.RedLightMaterialID`) (`self.YellowLightMaterialID`) (`self.GreenLightMaterialID`) (`self.TurnRedLightMaterialID`) (`self.TurnYellowLightMaterialID`) (`self.TurnGreenLightMaterialID`) (`self.RedLightMaterialSource`) (`self.YellowLightSource`) (`self.GreenLightSource`) (`self.TurnRedLightMaterialSource`) (`self.TurnYellowLightSource`) (`self.TurnGreenLightSource`)))
                  (:`then_3`
                    (set `/Game/AITraffic/TrafficLight_BP.FirstLightMaster` (`self.FirstLightMaster`) (`self.ForthLight`))
                    (set `/Game/AITraffic/TrafficLight_BP.SecondLight` (`self.SecondLight`) (`self.ForthLight`))
                    (set `/Game/AITraffic/TrafficLight_BP.ThirdLight` (`self.ThirdLight`) (`self.ForthLight`))
                    (set `/Game/AITraffic/TrafficLight_BP.ForthLight` _forthlight _forthlight)
                    (`self.DrawDebugLine` (`self.ForthLight`))
                    (`self.AutoSync` (`self.ForthLight`) (`self.LightDuration`) (`self.YellowLightDuration`) (`self.TurnLightDuration`) (`self.TrafficLightIntensity`) (`self.TrafficLightDelay`) (`self.RedLightMaterialID`) (`self.YellowLightMaterialID`) (`self.GreenLightMaterialID`) (`self.TurnRedLightMaterialID`) (`self.TurnYellowLightMaterialID`) (`self.TurnGreenLightMaterialID`) (`self.RedLightMaterialSource`) (`self.YellowLightSource`) (`self.GreenLightSource`) (`self.TurnRedLightMaterialSource`) (`self.TurnYellowLightSource`) (`self.TurnGreenLightSource`))))
                (else
                  (set `self.Auto Sync Master?` false))))
            (:`Is Not Valid`
              ;[1 0.2603 0.2703] Reset List.
              (`/Engine/EditorBlueprintResources/StandardMacros.IsValid` (`self.NorthLightMasterTemp`)
                (:`Is Valid`
                  (set `/Game/AITraffic/TrafficLight_BP.SecondLight` null _northlightmastertemp)
                  (set `/Game/AITraffic/TrafficLight_BP.ThirdLight` null _northlightmastertemp)
                  (set `/Game/AITraffic/TrafficLight_BP.ForthLight` null _northlightmastertemp))
                (:`Is Not Valid`
                  (set `self.SecondLight` null)
                  (set `self.ThirdLight` null)
                  (set `self.ForthLight` null)
                  (`SceneComponent.SetVisibility` (`self.MasterText`) false false) ; Turn off "Master" text.
                )))))
        (:`then_1`
          ;[1 0.4471 0.8829] Use Turn Signals and/or Turn box collision.
          (if (`self.UseTurnSignals?`)
            (`SceneComponent.SetVisibility` _turnlight true false)
            (else
              (`SceneComponent.SetVisibility` _turnlight false true)))
          (if (`self.UseSplines?`)
            (`SceneComponent.SetVisibility` _turnvehiclecollisionbox false false :!label _label)
            (elif (`self.UseTurnSignals?`)
              (goto _label)
              (else
                (`SceneComponent.SetVisibility` _turnvehiclecollisionbox true false)))))
        (:`then_2`
          ;[1 0.4836 0.899] Use box collision or not.
          (if (`self.UseSplines?`)
            (`SceneComponent.SetVisibility` _mainvehiclecollisionbox false false)
            (else
              (`SceneComponent.SetVisibility` _mainvehiclecollisionbox true false))))
        (:`then_3`
          ;[1 0.5437 0.08523] Public Transformations.
          (`SceneComponent.K2_SetRelativeTransform` (`self.MainVehicleCollisionBox`) (`KismetMathLibrary.MakeTransform` (`self.StopZoneLocation`) (`KismetMathLibrary.MakeRotator` 0.0 0.0 (`self.StopZoneRotation`)) (`self.StopZoneScale`)) false false) ; Set Public Transformations
          (`SceneComponent.K2_SetRelativeTransform` (`self.TurnVehicleCollisionBox`) (`KismetMathLibrary.MakeTransform` (`self.TurnZoneLocation`) (`KismetMathLibrary.MakeRotator` 0.0 0.0 (`self.TurnZoneRotation`)) (`self.TurnZoneScale`)) false false) ; Set Public Turn Transformations
        )))
    (:`then_1`
      (bind _returnvalue_4 (`PrimitiveComponent.CreateDynamicMaterialInstance` (`self.TurnLight`) (`self.TurnRedLightMaterialID`) (`self.TurnRedLightMaterialSource`) "None"))
      (set `self.TurnRedLightMaterial` _returnvalue_4)
      (bind _returnvalue_5 (`PrimitiveComponent.CreateDynamicMaterialInstance` (`self.TurnLight`) (`self.TurnYellowLightMaterialID`) (`self.TurnYellowLightSource`) "None"))
      (set `self.TurnYellowLightMaterial` _returnvalue_5)
      (bind _returnvalue_6 (`PrimitiveComponent.CreateDynamicMaterialInstance` (`self.TurnLight`) (`self.TurnGreenLightMaterialID`) (`self.TurnGreenLightSource`) "None"))
      (set `self.TurnGreenLightMaterial` _returnvalue_6))))