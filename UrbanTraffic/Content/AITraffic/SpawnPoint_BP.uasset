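; AI traffic spawn point that periodically spawns random cars from VehicleSetup, up to MaxSpawnCount or endlessly at -1.
; Tick drives a random Delay, then scans all AI_Car_Source actors and skips spawning if any is within 1000 units.
; Spawned cars inherit state, first waypoint and path, parking range and light settings.
; A random body material becomes a dynamic instance; only spawns with a valid material increment the counter.
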(event `self.ReceiveTick`
  (params (DeltaSeconds :type "Float (single-precision)"))
  (bind _rootcomponent (`self.RootComponent`))
  (bind _cars (break `/Game/AITraffic/Cars_Struct` (`self.VehicleSetup`)))
  (bind (_returnvalue_location _returnvalue_rotation) (`KismetMathLibrary.BreakTransform` (`SceneComponent.K2_GetComponentToWorld` _rootcomponent)))
  (bind _output (`|GetArrayItem` (`self.BodyMaterial`) (`KismetMathLibrary.RandomIntegerInRange` 0 (- (`KismetArrayLibrary.Array_Length` (`self.BodyMaterial`)) 1))))
  (bind _output_2 (`|GetArrayItem` _cars (`KismetMathLibrary.RandomIntegerInRange` 0 (- (`KismetArrayLibrary.Array_Length` _cars) 1))))
  (if (== (`self.MaxSpawnCount`) -1)
    (`KismetSystemLibrary.Delay` (`KismetMathLibrary.RandomFloatInRange` (`self.SpawnRandomMinRange`) (`self.SpawnRandomMaxRange`)) :!label _label)
    (if (`KismetSystemLibrary.IsValidClass` _output_2)
      (bind _outactors (`GameplayStatics.GetAllActorsOfClass` "/Game/AITraffic/AI_Car_Source.AI_Car_Source_C"))
      (for _array_element _outactors
        (if (<= (`KismetMathLibrary.Vector_Distance` (`SceneComponent.K2_GetComponentLocation` (`WheeledVehicle.Mesh` _array_element)) (`SceneComponent.K2_GetComponentLocation` _rootcomponent)) 1000.0)
          (set `self.SpawnerCleared?` false)))
      (if (`self.SpawnerCleared?`)
        (bind _returnvalue (`|SpawnActorFromClass` _output_2 (`KismetMathLibrary.MakeTransform` _returnvalue_location _returnvalue_rotation) "Undefined" "OverrideRootScale" null null))
        (`/Engine/EditorBlueprintResources/StandardMacros.IsValid` _returnvalue
          (:`Is Valid`
            (set `/Game/AITraffic/AI_Car_Source.State` (`self.State`) _returnvalue)
            (set `/Game/AITraffic/AI_Car_Source.FirstWaypoint` (`self.FirstWaypoint`) _returnvalue)
            (set `/Game/AITraffic/AI_Car_Source.FirstPath` (`self.FirstPath`) _returnvalue)
            (set `/Game/AITraffic/AI_Car_Source.HeadlightsOn?` (`self.HeadlightsOn?`) _returnvalue)
            (set `/Game/AITraffic/AI_Car_Source.ParkingSearchRange` (`self.ParkingSearchRange`) _returnvalue)
            (set `/Game/AITraffic/AI_Car_Source.TurnLightsIntensity` (`self.TurnLightsIntensity`) _returnvalue)
            (set `/Game/AITraffic/AI_Car_Source.BrakeLightIntensity` (`self.BrakeLightIntensity`) _returnvalue)
            (set `/Game/AITraffic/AI_Car_Source.HeadlightIntensity` (`self.Headlight Intensity`) _returnvalue)
            (set `/Game/AITraffic/AI_Car_Source.BrakeLightsMaterialID` (`self.BrakeLightsMaterialID`) _returnvalue)
            (set `/Game/AITraffic/AI_Car_Source.HeadlightsMaterialID` (`self.HeadlightsMaterialID`) _returnvalue)
            (set `/Game/AITraffic/AI_Car_Source.LeftTurnMaterialID` (`self.LeftTurnMaterialID`) _returnvalue)
            (set `/Game/AITraffic/AI_Car_Source.RightTurnMaterialID` (`self.RightTurnMaterialID`) _returnvalue)
            (set `/Game/AITraffic/AI_Car_Source.HeadlightsMaterial` (`self.HeadlightsMaterial`) _returnvalue)
            (set `/Game/AITraffic/AI_Car_Source.BrakeLightsMaterial` (`self.BrakeLightsMaterial`) _returnvalue)
            (set `/Game/AITraffic/AI_Car_Source.LeftTurnMaterial` (`self.LeftTurnMaterial`) _returnvalue)
            (set `/Game/AITraffic/AI_Car_Source.RightTurnMaterial` (`self.RightTurnMaterial`) _returnvalue)
            (`/Engine/EditorBlueprintResources/StandardMacros.IsValid` _output
              (:`Is Valid`
                (`PrimitiveComponent.CreateDynamicMaterialInstance` (`WheeledVehicle.Mesh` _returnvalue) (`self.BodyMaterialID`) _output "None")
                (bind _result (`/Engine/EditorBlueprintResources/StandardMacros.IncrementInt` (`self.SpawnCounter`))
                  (:`  `
                    (set `self.SpawnCounter` _result)))))))
        (else
          (set `self.SpawnerCleared?` true))))
    (elif (not (<= (`self.MaxSpawnCount`) (`self.SpawnCounter`)))
      (goto _label))))

(fn `UserConstructionScript`)