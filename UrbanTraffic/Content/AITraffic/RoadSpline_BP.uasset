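; Road spline actor for AI traffic that links to straight, right-turn and left-turn successor splines and an assigned traffic light.
; When UseDebugLine is on, its Construction Script draws color-coded debug lines from the spline's end to each valid successor's start and to the light's location.
; The event graph has no logic, so this Blueprint only holds the links and visualizes them.
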(event `self.ReceiveTick`
  (params (DeltaSeconds :type "Float (single-precision)")))

(fn `UserConstructionScript`
  (bind _spline (`self.Spline`))
  (bind _spline_2 (`self.Spline`))
  (bind _rightturn (`self.RightTurn`))
  (bind _spline_3 (`self.Spline`))
  (bind _leftturn (`self.LeftTurn`))
  (bind _assignedtrafficlight (`self.AssignedTrafficLight`))
  (bind _straight (`self.Straight`))
  (bind _spline_4 (`self.Spline`))
  (bind _spline_5 (`/Game/AITraffic/RoadSpline_BP.Spline` _rightturn))
  (bind _spline_6 (`/Game/AITraffic/RoadSpline_BP.Spline` _leftturn))
  (bind _spline_7 (`/Game/AITraffic/RoadSpline_BP.Spline` _straight))
  (bind _returnvalue (`SplineComponent.GetSplineLength` _spline_5))
  (bind _returnvalue_2 (`SplineComponent.GetSplineLength` _spline_6))
  (bind _returnvalue_3 (`SplineComponent.GetSplineLength` _spline_7))
  (if (`self.UseDebugLine?`)
    (`|ExecutionSequence`
      (:`then_0`
        (`/Engine/EditorBlueprintResources/StandardMacros.IsValid` _straight
          (:`Is Valid`
            (`KismetSystemLibrary.DrawDebugLine` (`SplineComponent.GetLocationAtDistanceAlongSpline` _spline_4 (`SplineComponent.GetSplineLength` _spline_4) "World") (`SplineComponent.GetLocationAtDistanceAlongSpline` _spline_7 (- _returnvalue_3 _returnvalue_3) "World") (struct :`R` 1.0 :`G` 0.699787 :`A` 1.0) (`self.BugLineDuration`) (`self.BugLineThickness`)))))
      (:`then_1`
        (`/Engine/EditorBlueprintResources/StandardMacros.IsValid` _rightturn
          (:`Is Valid`
            (`KismetSystemLibrary.DrawDebugLine` (`SplineComponent.GetLocationAtDistanceAlongSpline` _spline_2 (`SplineComponent.GetSplineLength` _spline_2) "World") (`SplineComponent.GetLocationAtDistanceAlongSpline` _spline_5 (- _returnvalue _returnvalue) "World") (struct :`R` 1.0 :`G` 0.084041 :`A` 1.0) (`self.BugLineDuration`) (`self.BugLineThickness`)))))
      (:`then_2`
        (`/Engine/EditorBlueprintResources/StandardMacros.IsValid` _leftturn
          (:`Is Valid`
            (`KismetSystemLibrary.DrawDebugLine` (`SplineComponent.GetLocationAtDistanceAlongSpline` _spline_3 (`SplineComponent.GetSplineLength` _spline_3) "World") (`SplineComponent.GetLocationAtDistanceAlongSpline` _spline_6 (- _returnvalue_2 _returnvalue_2) "World") (struct :`R` 0.204612 :`G` 1.0 :`A` 1.0) (`self.BugLineDuration`) (`self.BugLineThickness`)))))
      (:`then_3`
        (`/Engine/EditorBlueprintResources/StandardMacros.IsValid` _assignedtrafficlight
          (:`Is Valid`
            (`KismetSystemLibrary.DrawDebugLine` (`SplineComponent.GetLocationAtDistanceAlongSpline` _spline (`SplineComponent.GetSplineLength` _spline) "World") (`self.K2_GetActorLocation` _assignedtrafficlight) (struct :`R` 0.04144 :`G` 0.238863 :`B` 1.0 :`A` 1.0) (`self.BugLineDuration`) (`self.BugLineThickness`))))))))